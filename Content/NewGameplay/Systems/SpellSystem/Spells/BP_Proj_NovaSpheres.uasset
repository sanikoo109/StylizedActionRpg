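; Nova spell projectile actor that bursts a ring of sphere projectiles outward and damages actors it overlaps.
; On BeginPlay it adds evenly yawed sphere components with attached particle effects, launches them along their forward vectors after a brief delay, and later deactivates the effects.
; Overlaps skip the instigator and use an AddUnique array so each actor takes damage only once across all spheres.
; Logic to ignore the instigator during movement is present but disconnected.
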(event Collision|EventActorBeginOverlap
  (params (OtherActor :type Actor%20Object%20Reference))
  (bind _returnvalue (Game|GetInstigator))
  (if (!= OtherActor (Game|GetInstigator))
    (bind _returnvalue_2 (Utilities|Array|AddUnique (Variables|Default|GetDamagedActors) OtherActor))
    (Utilities|IsValidID _returnvalue_2
      (:Is%20Valid
        (Class|GameDamageInterface|ApplyGameDamage(Message) OtherActor (Variables|Default|GetDamage) (Pawn|GetController _returnvalue) _returnvalue false "0, 0, 0")))))

(event EventBeginPlay
  (Utilities|FlowControl|Sequence
    (:then_0
      (bind _index (Utilities|SimpleLoop (Variables|Default|GetProjectilesCount))
        (:LoopBody
          (bind _returnvalue (AddComponent|AddSphereComponent false (Math|Transform|MakeTransform "0, 0, 0" (Math|Rotator|MakeRotator 0.0 0.0 (* (/ (Math|Conversions|ToFloat(Integer) _index) (Math|Conversions|ToFloat(Integer) (Variables|Default|GetProjectilesCount))) 3.6e+02)))))
          (bind _returnvalue_2 (AddComponent|AddParticleSystemComponent false))
          (Effects|Components|ParticleSystem|SetTemplate _returnvalue_2 (Variables|Default|GetEffect))
          (Transformation|AttachComponentToComponent _returnvalue_2 _returnvalue "None" "KeepRelative" "KeepRelative" "KeepRelative" true))))
    (:then_1
      (Utilities|FlowControl|Delay 0.05)
      (for _array_element (Actor|GetComponentsByClass "/Script/Engine.SphereComponent")
        (Physics|AddImpulse _array_element (* (Math|Vector|GetForwardVector _array_element) 1e+03) "None" true)))
    (:then_2
      (Utilities|FlowControl|Delay 1.0)
      (for _array_element_2 (Actor|GetComponentsByClass "/Script/Engine.ParticleSystemComponent")
        (Components|Activation|Deactivate _array_element_2)))))

(fn ConstructionScript)