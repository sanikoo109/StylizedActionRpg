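; BP_Room is a room actor in the room system that records the player's first visit and announces it through an OnVisit dispatcher.
; It listens for overlaps on a referenced Trigger actor, filters for Char_Player, and also checks for a player already inside at BeginPlay.
; Visit uses a Visited flag to broadcast only once.
; The room's own OnVisit handler is an empty stub.
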(event Custom|OnActorBeginOverlap_Event
  (params (OverlappedActor :type Actor%20Object%20Reference) (OtherActor :type Actor%20Object%20Reference))
  (Utilities|Casting|CastToChar_Player OtherActor)
  (CallFunction|Visit))

(event Custom|OnVisit_Event)

(event EventBeginPlay
  (EventDispatchers|AssignOnActorBeginOverlap (Variables|Default|GetTrigger) (delegate Custom|OnActorBeginOverlap_Event))
  (EventDispatchers|BindEventtoOnVisit (delegate Custom|OnVisit_Event))
  (if (Utilities|Array|IsNotEmpty (Collision|GetOverlappingActors (Variables|Default|GetTrigger) "/Game/NewGameplay/Characters/Player/Char_Player.Char_Player_C" :!class /Script/Engine.Actor))
    (CallFunction|Visit)))

(event Collision|EventActorBeginOverlap
  (params (OtherActor :type Actor%20Object%20Reference)))

(event EventTick
  (params (DeltaSeconds :type Float%20%28single-precision%29)))

(fn ConstructionScript)

(fn Visit
  (if (not (Variables|Default|GetbVisited))
    (Variables|Default|SetbVisited true)
    (Default|CallOnVisit)))