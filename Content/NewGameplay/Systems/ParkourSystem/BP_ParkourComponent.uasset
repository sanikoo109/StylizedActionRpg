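; Parkour component Blueprint that handles the animation side of ladder climbing and ledge-hang climb-ups, standing or crouched, for its parent character.
; Ladder montage sections act as a state machine, selecting alternating left/right steps, exits and busy checks.
; Montage notifies and endings drive ladder position and ledge state callbacks, with crouch state updates staggered by zero-length delays.
; The CrouchAlpha curve blends capsule half-height while re-seating the mesh.
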(event EventBeginPlay)

(event EventTick
  (params (DeltaSeconds :type Float%20%28single-precision%29)))

(event EventBeginLadderEvent
  (bind _notifyname (Animation|Montage|PlayMontage (Variables|/Script/Engine.Character|GetMesh (Variables|Default|GetParentCharacter)) "/Game/Characters/Mannequins/Animations/Manny/Ladder_Montage.Ladder_Montage" 1.0 0.0 "Init")
    (:OnCompleted
      (Class|ParkourComponent|LadderAnimEnded :!label _label))
    (:OnInterrupted
      (goto _label))
    (:OnNotifyBegin
      (switch name _notifyname
        (:UpdatePos
          (Class|ParkourComponent|UpdateLadderPos))))))

(event EventPlayMontageLedgeHangUp
  (Class|MyCharacter|ForceAlignEnd (Variables|Default|GetParentCharacter))
  (Animation|Montage|PlayMontage (Variables|/Script/Engine.Character|GetMesh (Variables|Default|GetParentCharacter)) "/Game/Characters/Mannequins/Animations/Manny/LedgeHang/LedgeHang_Up_Montage.LedgeHang_Up_Montage"
    (:OnBlendOut
      _)
    (:OnInterrupted
      _))
  (Class|ParkourComponent|EndMontageLedgeHangUp))

(event EventPlayMontageLedgeHangUpCrouch
  (Class|MyCharacter|ForceAlignEnd (Variables|Default|GetParentCharacter))
  (bind _notifyname (Animation|Montage|PlayMontage (Variables|/Script/Engine.Character|GetMesh (Variables|Default|GetParentCharacter)) "/Game/Characters/Mannequins/Animations/Manny/LedgeHang/LedgeHang_UpCrouch_Montage.LedgeHang_UpCrouch_Montage")
    (:OnInterrupted
      (Class|ParkourComponent|EndMontageLedgeHangUpCrouch))
    (:OnNotifyBegin
      (switch name _notifyname
        (:UpdateHeight
          (Class|ParkourComponent|SetUpdatingHeight true))
        (:UpdateState
          (Class|ParkourComponent|LedgeHangUpCrouchUpdateState)
          (Utilities|FlowControl|Delay 0.0)
          (Class|ParkourComponent|LedgeHangUpCrouchUpdateState 1)
          (Utilities|FlowControl|Delay 0.0)
          (Class|ParkourComponent|LedgeHangUpCrouchUpdateState 2))))
    (:OnNotifyEnd
      (switch name _notifyname
        (:UpdateHeight
          (Class|ParkourComponent|SetUpdatingHeight false))))))

(event EventLadderExitDown
  (Ability|Animation|MontageJumptoSection (Components|SkeletalMesh|GetAnimInstance (Variables|/Script/Engine.Character|GetMesh (Variables|Default|GetParentCharacter))) "Exit_Down" "/Game/Characters/Mannequins/Animations/Manny/Ladder_Montage.Ladder_Montage"))

(event EventLadderExitUp
  (Ability|Animation|MontageJumptoSection (Components|SkeletalMesh|GetAnimInstance (Variables|/Script/Engine.Character|GetMesh (Variables|Default|GetParentCharacter))) "Exit_Up" "/Game/Characters/Mannequins/Animations/Manny/Ladder_Montage.Ladder_Montage"))

(event EventLadderPlayStepAnim
  (params (bUp :type Boolean))
  (bind _parentcharacter (Variables|Default|GetParentCharacter))
  (bind _mesh (Variables|/Script/Engine.Character|GetMesh _parentcharacter))
  (bind _returnvalue (Components|SkeletalMesh|GetAnimInstance _mesh))
  (bind _returnvalue_2 (Animation|Montage|MontageGetCurrentSection _returnvalue "/Game/Characters/Mannequins/Animations/Manny/Ladder_Montage.Ladder_Montage"))
  (bind _returnvalue_3 (== _returnvalue_2 "R_Idle"))
  (Ability|Animation|MontageJumptoSection _returnvalue (select bUp (select _returnvalue_3 "ToL" "ToR") (select _returnvalue_3 "ToL_Reverse" "ToR_Reverse")) "/Game/Characters/Mannequins/Animations/Manny/Ladder_Montage.Ladder_Montage"))

(event EventLadderStopMontage
  (Animation|Montage|MontageStop (Components|SkeletalMesh|GetAnimInstance (Variables|/Script/Engine.Character|GetMesh (Variables|Default|GetParentCharacter))) 0.0 "/Game/Characters/Mannequins/Animations/Manny/Ladder_Montage.Ladder_Montage"))

(event EventUpdateHeightbyAnimCurve
  (bind _asbp_my_character (Utilities|Casting|CastToBP_MyCharacter (Variables|Default|GetParentCharacter)))
  (Default|SetHalfHeightRelativeFloor _asbp_my_character (Math|Float|Lerp (Variables|Default|GetCapsuleDefaultHalfHeight) (Variables|/Script/Engine.CharacterMovementComponent|GetCrouchedHalfHeight (Variables|/Script/Engine.Character|GetCharacterMovement (Variables|Default|GetParentCharacter))) (Animation|Curves|GetCurveValue (Components|SkeletalMesh|GetAnimInstance (Variables|/Script/Engine.Character|GetMesh (Variables|Default|GetParentCharacter))) "CrouchAlpha")))
  (Transformation|SetRelativeLocation (Variables|/Script/Engine.Character|GetMesh (Variables|Default|GetParentCharacter)) (Math|Vector|MakeVector 0.0 0.0 (* (Components|Capsule|GetUnscaledCapsuleHalfHeight (Variables|/Script/Engine.Character|GetCapsuleComponent (Variables|Default|GetParentCharacter))) -1.0)) false true))

(fn IsLadderBusy
  (bind _parentcharacter (Variables|Default|GetParentCharacter))
  (bind _mesh (Variables|/Script/Engine.Character|GetMesh _parentcharacter))
  (bind _returnvalue (Components|SkeletalMesh|GetAnimInstance _mesh))
  (bind _returnvalue_2 (Animation|Montage|MontageGetCurrentSection _returnvalue "/Game/Characters/Mannequins/Animations/Manny/Ladder_Montage.Ladder_Montage"))
  (return (Math|Boolean|ORBoolean (== _returnvalue_2 "ToR") (== _returnvalue_2 "ToL") (== _returnvalue_2 "Init") (== _returnvalue_2 "ToR_Reverse") (== _returnvalue_2 "ToL_Reverse") (== _returnvalue_2 "Exit_Up") (== _returnvalue_2 "Exit_Down"))))

(fn IsPlayingLedgeHangUpAnim
  (return (Animation|Montage|MontageIsPlaying (Components|SkeletalMesh|GetAnimInstance (Variables|/Script/Engine.Character|GetMesh (Variables|Default|GetParentCharacter))) "/Game/Characters/Mannequins/Animations/Manny/LedgeHang/LedgeHang_Up_Montage.LedgeHang_Up_Montage")))