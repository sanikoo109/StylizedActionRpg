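; Character combat component that plays attack and reload montages on the character and weapon mesh, with helpers for weapon lookup and trace points.
; Montage notifies toggle left/right attack traces, cast DT_Spells spells from configured sockets or aim, fire projectiles scaled by the Tension curve, and consume ammo.
; Attack release stops montages or jumps to numbered End sections.
; Weapon trails use DoOnce with a retriggerable delay, ending when calls stop.
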(event EventTick
  (params (DeltaSeconds :type Float%20%28single-precision%29)))

(event EventCheckBlockingNextFrame
  (Utilities|FlowControl|Delay 0.0)
  (Class|CombatComponent|CheckBlocking))

(event EventItemAttackEvent
  (params (MontageToPlay :type Anim%20Montage%20Object%20Reference) (PlayRate :type Float%20%28single-precision%29))
  (Utilities|IsValid MontageToPlay
    (:Is%20Valid
      (bind _asskeletal_mesh_component (Utilities|Casting|CastToSkeletalMeshComponent (Default|GetWeaponMesh (.AsBP%20My%20Character (Utilities|Casting|CastToBP_MyCharacter (Variables|Default|GetParentChar))) true)))
      (Animation|Montage|PlayMontage _asskeletal_mesh_component MontageToPlay PlayRate))))

(event EventPlayReloadAnimChar
  (params (MontageToPlay :type Anim%20Montage%20Object%20Reference) (PlayRate :type Float%20%28single-precision%29))
  (bind _notifyname (Animation|Montage|PlayMontage (Class|CombatComponent|GetCharMesh) MontageToPlay PlayRate)
    (:OnBlendOut
      (Class|CombatComponent|ReloadEnd :!label _label))
    (:OnInterrupted
      (goto _label))
    (:OnNotifyBegin
      (switch name _notifyname
        (:Reload
          (Class|CombatComponent|ReloadExecute))
        (:ShowAmmo
          (Class|CombatComponent|SetShowReloadAmmo true))))))

(event EventPlayReloadAnimItem
  (params (MontageToPlay :type Anim%20Montage%20Object%20Reference) (PlayRate :type Float%20%28single-precision%29))
  (Utilities|IsValid MontageToPlay
    (:Is%20Valid
      (bind _asbp_my_character (Utilities|Casting|CastToBP_MyCharacter (Variables|Default|GetParentChar)))
      (bind _asskeletal_mesh_component (Utilities|Casting|CastToSkeletalMeshComponent (Default|GetWeaponMesh _asbp_my_character true)))
      (Animation|Montage|PlayMontage _asskeletal_mesh_component MontageToPlay PlayRate))))

(event EventAttackCast
  (bind _parentchar (Variables|Default|GetParentChar))
  (bind _parentchar_2 (Variables|Default|GetParentChar))
  (bind _asbp_my_character (Utilities|Casting|CastToBP_MyCharacter _parentchar_2))
  (bind _asbp_my_character_2 (Utilities|Casting|CastToBP_MyCharacter _parentchar))
  (bind _result (Default|GetAimTransform _asbp_my_character))
  (bind _result_2 (Default|GetAttackMesh _asbp_my_character_2 true))
  (bind _mesh (Variables|/Script/Engine.Character|GetMesh _asbp_my_character_2))
  (bind (_location _rotation) (Math|Transform|BreakTransform _result))
  ;[0.15 0.15 0.15 0.5] Cast spell
  (bind _returnvalue (Utilities|GetDataTableRow "/Game/NewGameplay/Systems/SpellSystem/DT_Spells.DT_Spells" (Utilities|Struct|BreakCombatAttackData (Variables|Default|GetCombatAttackData)))
    (:then
      (Default|CallOnCastSpell (Utilities|Struct|BreakCombatAttackData (Variables|Default|GetCombatAttackData)) (Math|Transform|MakeTransform (Utilities|Select :Index (.MeshTarget (Utilities|Struct|BreakSpellSocketData (.SocketName (Utilities|Struct|BreakSpellTableData _returnvalue)))) :ESMT_None (Class|CombatComponent|GetSocketLocationSafe (Utilities|Select :Index (.MeshTarget (Utilities|Struct|BreakSpellSocketData (.SocketName (Utilities|Struct|BreakSpellTableData _returnvalue)))) :ESMT_None 0 :ESMT_Auto _result_2 :ESMT_Char _mesh :ESMT_Aim 0) (.Socket (Utilities|Struct|BreakSpellSocketData (.SocketName (Utilities|Struct|BreakSpellTableData _returnvalue))))) :ESMT_Auto (Class|CombatComponent|GetSocketLocationSafe (Utilities|Select :Index (.MeshTarget (Utilities|Struct|BreakSpellSocketData (.SocketName (Utilities|Struct|BreakSpellTableData _returnvalue)))) :ESMT_None 0 :ESMT_Auto _result_2 :ESMT_Char _mesh :ESMT_Aim 0) (.Socket (Utilities|Struct|BreakSpellSocketData (.SocketName (Utilities|Struct|BreakSpellTableData _returnvalue))))) :ESMT_Char (Class|CombatComponent|GetSocketLocationSafe (Utilities|Select :Index (.MeshTarget (Utilities|Struct|BreakSpellSocketData (.SocketName (Utilities|Struct|BreakSpellTableData _returnvalue)))) :ESMT_None 0 :ESMT_Auto _result_2 :ESMT_Char _mesh :ESMT_Aim 0) (.Socket (Utilities|Struct|BreakSpellSocketData (.SocketName (Utilities|Struct|BreakSpellTableData _returnvalue))))) :ESMT_Aim _location) (Utilities|Select :Index (.MeshTarget (Utilities|Struct|BreakSpellSocketData (.RotationSocketName (Utilities|Struct|BreakSpellTableData _returnvalue)))) :ESMT_None (Class|CombatComponent|GetSocketRotationSafe (Utilities|Select :Index (.MeshTarget (Utilities|Struct|BreakSpellSocketData (.RotationSocketName (Utilities|Struct|BreakSpellTableData _returnvalue)))) :ESMT_None 0 :ESMT_Auto _result_2 :ESMT_Char _mesh :ESMT_Aim 0) (.Socket (Utilities|Struct|BreakSpellSocketData (.RotationSocketName (Utilities|Struct|BreakSpellTableData _returnvalue))))) :ESMT_Auto (Class|CombatComponent|GetSocketRotationSafe (Utilities|Select :Index (.MeshTarget (Utilities|Struct|BreakSpellSocketData (.RotationSocketName (Utilities|Struct|BreakSpellTableData _returnvalue)))) :ESMT_None 0 :ESMT_Auto _result_2 :ESMT_Char _mesh :ESMT_Aim 0) (.Socket (Utilities|Struct|BreakSpellSocketData (.RotationSocketName (Utilities|Struct|BreakSpellTableData _returnvalue))))) :ESMT_Char (Class|CombatComponent|GetSocketRotationSafe (Utilities|Select :Index (.MeshTarget (Utilities|Struct|BreakSpellSocketData (.RotationSocketName (Utilities|Struct|BreakSpellTableData _returnvalue)))) :ESMT_None 0 :ESMT_Auto _result_2 :ESMT_Char _mesh :ESMT_Aim 0) (.Socket (Utilities|Struct|BreakSpellSocketData (.RotationSocketName (Utilities|Struct|BreakSpellTableData _returnvalue))))) :ESMT_Aim _rotation)) (Utilities|Select :Index (.MeshTarget (Utilities|Struct|BreakSpellSocketData (.PreviewSocketName (Utilities|Struct|BreakSpellTableData _returnvalue)))) :ESMT_None (Class|CombatComponent|GetSocketTransformSafe (Utilities|Select :Index (.MeshTarget (Utilities|Struct|BreakSpellSocketData (.PreviewSocketName (Utilities|Struct|BreakSpellTableData _returnvalue)))) :ESMT_None 0 :ESMT_Auto _result_2 :ESMT_Char _mesh :ESMT_Aim 0) (.Socket (Utilities|Struct|BreakSpellSocketData (.PreviewSocketName (Utilities|Struct|BreakSpellTableData _returnvalue))))) :ESMT_Auto (Class|CombatComponent|GetSocketTransformSafe (Utilities|Select :Index (.MeshTarget (Utilities|Struct|BreakSpellSocketData (.PreviewSocketName (Utilities|Struct|BreakSpellTableData _returnvalue)))) :ESMT_None 0 :ESMT_Auto _result_2 :ESMT_Char _mesh :ESMT_Aim 0) (.Socket (Utilities|Struct|BreakSpellSocketData (.PreviewSocketName (Utilities|Struct|BreakSpellTableData _returnvalue))))) :ESMT_Char (Class|CombatComponent|GetSocketTransformSafe (Utilities|Select :Index (.MeshTarget (Utilities|Struct|BreakSpellSocketData (.PreviewSocketName (Utilities|Struct|BreakSpellTableData _returnvalue)))) :ESMT_None 0 :ESMT_Auto _result_2 :ESMT_Char _mesh :ESMT_Aim 0) (.Socket (Utilities|Struct|BreakSpellSocketData (.PreviewSocketName (Utilities|Struct|BreakSpellTableData _returnvalue))))) :ESMT_Aim _result)))))

(event EventShowTrailR
  (Utilities|FlowControl|Sequence
    (:then_0
      (Utilities|FlowControl|DoOnce false :!label _label
        (:Completed
          (Effects|Particles|Trails|BeginTrails (Default|GetWeaponTrail (.AsBP%20My%20Character (Utilities|Casting|CastToBP_MyCharacter (Variables|Default|GetParentChar))) true) "Damage_Start" "Damage_End" "ETrailWidthMode_FromCentre" 1.0))))
    (:then_1
      (Utilities|FlowControl|RetriggerableDelay 0.05)
      (Effects|Particles|Trails|EndTrails (Default|GetWeaponTrail (.AsBP%20My%20Character (Utilities|Casting|CastToBP_MyCharacter (Variables|Default|GetParentChar))) true))
      (goto _label Reset))))

(event EventShowTrailL
  (Utilities|FlowControl|Sequence
    (:then_0
      (Utilities|FlowControl|DoOnce false :!label _label
        (:Completed
          (Effects|Particles|Trails|BeginTrails (Default|GetWeaponTrail (.AsBP%20My%20Character (Utilities|Casting|CastToBP_MyCharacter (Variables|Default|GetParentChar))) false) "Damage_Start" "Damage_End" "ETrailWidthMode_FromCentre" 1.0))))
    (:then_1
      (Utilities|FlowControl|RetriggerableDelay 0.05)
      (Effects|Particles|Trails|EndTrails (Default|GetWeaponTrail (.AsBP%20My%20Character (Utilities|Casting|CastToBP_MyCharacter (Variables|Default|GetParentChar))) false))
      (goto _label Reset))))

(event EventAttackEvent
  (params (MontageToPlay :type Anim%20Montage%20Object%20Reference) (PlayRate :type Float%20%28single-precision%29))
  (bind _notifyname (Animation|Montage|PlayMontage (Class|CombatComponent|GetCharMesh) MontageToPlay PlayRate)
    (:OnCompleted
      (Class|CombatComponent|AttackEndAnim :!label _label))
    (:OnInterrupted
      (goto _label))
    (:OnNotifyBegin
      (switch name _notifyname
        (:TraceL
          (Class|CombatComponent|SetAttackTraceActive false true))
        (:TraceR
          (Class|CombatComponent|SetAttackTraceActive true true))
        (:Cast
          (Class|CombatComponent|AttackCast))
        (:Shoot
          (Class|CombatComponent|AttackShoot))
        (:ShowAmmo
          (Class|CombatComponent|SetShowAmmo true))))
    (:OnNotifyEnd
      (switch name _notifyname
        (:TraceL
          (Class|CombatComponent|SetAttackTraceActive false false))
        (:TraceR
          (Class|CombatComponent|SetAttackTraceActive true false))))))

(event EventAttackReleaseAction
  (params (ID :type Integer))
  (bind _returnvalue (Utilities|String|ToString(Integer) ID))
  (bind _returnvalue_2 (Utilities|String|Append "End_" _returnvalue))
  (bind _returnvalue_3 (Utilities|String|StringToName _returnvalue_2))
  (Ability|Animation|MontageJumptoSection (Class|CombatComponent|GetAnimInstance) _returnvalue_3 0)
  (bind _asskeletal_mesh_component (Utilities|Casting|CastToSkeletalMeshComponent (Default|GetWeaponMesh (.AsBP%20My%20Character (Utilities|Casting|CastToBP_MyCharacter (Variables|Default|GetParentChar))) true)))
  (Utilities|IsValid (Components|SkeletalMesh|GetAnimInstance _asskeletal_mesh_component)
    (:Is%20Valid
      (Ability|Animation|MontageJumptoSection (Components|SkeletalMesh|GetAnimInstance _asskeletal_mesh_component) _returnvalue_3 0))))

(event EventAttackReleaseBegin
  (params (ID :type Integer))
  (Animation|Montage|MontageStop (Class|CombatComponent|GetAnimInstance) 0.25 0)
  (bind _asskeletal_mesh_component (Utilities|Casting|CastToSkeletalMeshComponent (Default|GetWeaponMesh (.AsBP%20My%20Character (Utilities|Casting|CastToBP_MyCharacter (Variables|Default|GetParentChar))) true)))
  (Animation|Montage|MontageStop (Components|SkeletalMesh|GetAnimInstance _asskeletal_mesh_component) 0.25 0))

(event EventAttackShoot
  (bind _parentchar (Variables|Default|GetParentChar))
  (bind _returnvalue (Actor|GetComponentbyClass _parentchar "/Game/NewGameplay/Systems/InventorySystem/BP_InventoryComponent.BP_InventoryComponent_C"))
  (bind _returnvalue_2 (Default|GetSelectedSlotItem _returnvalue "EIST_WeaponL"))
  ;[0.15 0.15 0.15 0.5] Shoot
  (Utilities|FlowControl|Sequence
    (:then_0
      (Utilities|Struct|SetmembersinCombatAttackData (Variables|Default|GetCombatAttackData) false)
      (Class|CombatComponent|CheckCombatAttackData))
    (:then_1
      (Utilities|IsValid _returnvalue_2
        (:Is%20Valid
          (Game|SpawnActorfromClass (.ProjectileClass (Utilities|Struct|BreakInventoryItemTableData (Variables|/Game/NewGameplay/Systems/InventorySystem/BP_InventoryItem.BP_InventoryItem_C|GetItemTableData _returnvalue_2))) (Default|GetAimTransform (.AsBP%20My%20Character (Utilities|Casting|CastToBP_MyCharacter (Variables|Default|GetParentChar)))) "AlwaysSpawn" "MultiplyWithRoot" 0 1e+01 (Class|CombatComponent|GetDamage) true (Transformation|GetWorldTransform (Default|GetAmmoMesh (.AsBP%20My%20Character (Utilities|Casting|CastToBP_MyCharacter (Variables|Default|GetParentChar))))) (Animation|Curves|GetCurveValue (Class|CombatComponent|GetAnimInstance) "Tension") (Variables|Default|GetParentChar))
          (Default|WasteAmmo (Default|GetSelectedSlotItem (Actor|GetComponentbyClass (Variables|Default|GetParentChar) "/Game/NewGameplay/Systems/InventorySystem/BP_InventoryComponent.BP_InventoryComponent_C") "EIST_WeaponR") _returnvalue_2))))))

(event EventReloadExecute
  ;[0.15 0.15 0.15 0.5] Reload
  (Class|CombatComponent|SetShowReloadAmmo false)
  (Default|AddCount (Default|GetSelectedSlotItem (Actor|GetComponentbyClass (Variables|Default|GetParentChar) "/Game/NewGameplay/Systems/InventorySystem/BP_InventoryComponent.BP_InventoryComponent_C") "EIST_WeaponL") -1)
  (Default|Reload (Default|GetSelectedSlotItem (Actor|GetComponentbyClass (Variables|Default|GetParentChar) "/Game/NewGameplay/Systems/InventorySystem/BP_InventoryComponent.BP_InventoryComponent_C") "EIST_WeaponR")))

(fn GetCurrentWeapon
  (return (Default|GetSelectedSlotItem (Actor|GetComponentbyClass (Variables|Default|GetParentChar) "/Game/NewGameplay/Systems/InventorySystem/BP_InventoryComponent.BP_InventoryComponent_C") "EIST_WeaponR")))

(fn ReloadFunc
  (bind _attackspeed (Variables|Default|GetAttackSpeed))
  (bind _parentchar (Variables|Default|GetParentChar))
  (bind _parentchar_2 (Variables|Default|GetParentChar))
  (bind _returnvalue (Actor|GetComponentbyClass _parentchar "/Game/NewGameplay/Systems/InventorySystem/BP_InventoryComponent.BP_InventoryComponent_C"))
  (bind _returnvalue_2 (Actor|GetComponentbyClass _parentchar_2 "/Game/NewGameplay/Systems/InventorySystem/BP_InventoryComponent.BP_InventoryComponent_C"))
  (bind _returnvalue_3 (Default|GetSelectedSlotItem _returnvalue "EIST_WeaponL"))
  (bind _returnvalue_4 (Default|GetSelectedSlotItem _returnvalue_2 "EIST_WeaponR"))
  (bind _itemtabledata (Variables|/Game/NewGameplay/Systems/InventorySystem/BP_InventoryItem.BP_InventoryItem_C|GetItemTableData _returnvalue_4))
  (bind (_ammo _reloadmontage _reloadrate _reloaditemmontage) (Utilities|Struct|BreakInventoryItemTableData _itemtabledata))
  (bind _returnvalue_5 (* _reloadrate _attackspeed))
  (if (not (Animation|Montage|MontageIsPlaying (Class|CombatComponent|GetAnimInstance) 0))
    (Utilities|IsValid _returnvalue_4
      (:Is%20Valid
        (if (Default|CanReload _returnvalue_4)
          (Utilities|IsValid _returnvalue_3
            (:Is%20Valid
              (if (== _ammo (Variables|/Game/NewGameplay/Systems/InventorySystem/BP_InventoryItem.BP_InventoryItem_C|GetItemRowName _returnvalue_3))
                (Class|CombatComponent|SetReloading true)
                (Class|CombatComponent|PlayReloadAnimChar _reloadmontage _returnvalue_5)
                (Class|CombatComponent|PlayReloadAnimItem _reloaditemmontage _returnvalue_5)))))))))

(fn Reload
  (CallFunction|ReloadFunc))

(fn GetCurrentWeaponCauserFunc
  (for _array_element (Actor|GetComponentsByClass (Variables|Default|GetParentChar) "/Game/NewGameplay/Systems/InventorySystem/BP_DIC_ItemSlot.BP_DIC_ItemSlot_C")
    (if (Utilities|Enum|Equal(Enum) (Variables|/Script/NewGameplay.DIC_ItemSlot|GetSlot _array_element) "EIST_WeaponR")
      (bind _currentitem (Variables|/Game/NewGameplay/Systems/InventorySystem/BP_DesignItemComponent.BP_DesignItemComponent_C|GetCurrentItem _array_element)
        (:then
          (return _currentitem))
        (:else))))
  (return (Variables|Default|GetParentChar)))

(fn GetCurrentWeaponCauser
  (return (CallFunction|GetCurrentWeaponCauserFunc)))

(fn GetWeaponTracePoint
  (params (bEnd :type Boolean))
  (return (Class|CombatComponent|GetSocketLocationSafe (Default|GetWeaponMesh (.AsBP%20My%20Character (Utilities|Casting|CastToBP_MyCharacter (Variables|Default|GetParentChar))) true) (Utilities|String|SelectName "Damage_End" "Damage_Start" bEnd))))

(fn GetWeaponItem
  (return (Default|GetSelectedSlotItem (Actor|GetComponentbyClass (Variables|Default|GetParentChar) "/Game/NewGameplay/Systems/InventorySystem/BP_InventoryComponent.BP_InventoryComponent_C") "EIST_WeaponR")))

(fn GetSpellMove
  (params (Spell :type Name :default "None"))
  (bind _returnvalue (Utilities|GetDataTableRow "/Game/NewGameplay/Systems/SpellSystem/DT_Spells.DT_Spells" Spell)
    (:then
      (return (.Value (Utilities|Map|Find (Variables|Default|GetSpellCastMove) (Utilities|Struct|BreakSpellTableData _returnvalue))) true))
    (:RowNotFound
      (return "None" false))))

(fn GetWeaponMesh
  (Utilities|FlowControl|Sequence
    (:then_0
      (bind _asbp_my_character (Utilities|Casting|CastToBP_MyCharacter (Variables|Default|GetParentChar)))
      (bind _asskeletal_mesh_component (Utilities|Casting|CastToSkeletalMeshComponent (Default|GetWeaponMesh _asbp_my_character true)))
      (return _asskeletal_mesh_component))
    (:then_1
      (return 0))))