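; BP_ItemDesign_Skeletal is an inventory item display actor that shows an item's design as a skeletal mesh.
; When DesignItemLogicComp reports a new parent item, it applies that item's design mesh and anim instance class from its table data, or clears both if the item is invalid.
; Item design interface functions toggle actor visibility and expose the logic component and ItemMesh, which also serves as the ammo mesh.
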(event OnUpdateParentItem(DesignItemLogicComp)
  (params (NewItem :type Inventory%20Item%20Object%20Reference) (PrevItem :type Inventory%20Item%20Object%20Reference))
  (bind _itemtabledata (Variables|/Game/NewGameplay/Systems/InventorySystem/BP_InventoryItem.BP_InventoryItem_C|GetItemTableData NewItem))
  (bind (_designmesh _animinstanceclass) (Utilities|Struct|BreakInventoryItemTableData _itemtabledata))
  (Utilities|IsValid NewItem
    (:Is%20Valid
      (Components|SkeletalMesh|SetSkeletalMeshAsset (Variables|Default|GetItemMesh) _designmesh)
      (Components|SkeletalMesh|SetAnimInstanceClass (Variables|Default|GetItemMesh) _animinstanceclass))
    (:Is%20Not%20Valid
      (Components|SkeletalMesh|SetSkeletalMeshAsset (Variables|Default|GetItemMesh) 0)
      (Components|SkeletalMesh|SetAnimInstanceClass (Variables|Default|GetItemMesh) 0))))

(event EventIItemDesignUpdateVisible
  (params (IsVisible :type Boolean))
  (Rendering|SetActorHiddenInGame (not IsVisible)))

(fn ConstructionScript)

(fn IItemDesignGetAmmoMesh
  (return (Variables|Default|GetItemMesh)))

(fn IItemDesignGetLogicComp
  (return (Variables|Default|GetDesignItemLogicComp)))

(fn IItemDesignGetMesh
  (return (Variables|Default|GetItemMesh)))