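; Static-mesh item design actor that provides the visual representation of an inventory item.
; When its design logic component reports a parent item change, it applies the single or multiple pickup mesh from the item's table data, or clears the mesh if the item is invalid.
; The item design interface toggles visibility and exposes the logic component and mesh, with the same mesh doubling as the ammo mesh.
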(event OnUpdateParentItem(BP_DesignItemLogicComp)
  (params (NewItem :type Inventory%20Item%20Object%20Reference) (PrevItem :type Inventory%20Item%20Object%20Reference))
  (bind _itemtabledata (Variables|/Game/NewGameplay/Systems/InventorySystem/BP_InventoryItem.BP_InventoryItem_C|GetItemTableData NewItem))
  (bind (_pickupmesh _pickupmesh_multiple) (Utilities|Struct|BreakInventoryItemTableData _itemtabledata))
  (Utilities|IsValid NewItem
    (:Is%20Valid
      (Components|StaticMesh|SetStaticMesh (Variables|Default|GetItemMesh) (select (Variables|/Game/NewGameplay/Systems/InventorySystem/BP_DesignItemLogicComp.BP_DesignItemLogicComp_C|GetbShowMultipleMesh (Variables|Default|GetBP_DesignItemLogicComp)) _pickupmesh_multiple _pickupmesh)))
    (:Is%20Not%20Valid
      (Components|StaticMesh|SetStaticMesh (Variables|Default|GetItemMesh) 0))))

(event EventIItemDesignUpdateVisible
  (params (IsVisible :type Boolean))
  (Rendering|SetActorHiddenInGame (not IsVisible)))

(fn ConstructionScript)

(fn IItemDesignGetAmmoMesh
  (return (Variables|Default|GetItemMesh)))

(fn IItemDesignGetLogicComp
  (return (Variables|Default|GetBP_DesignItemLogicComp)))

(fn IItemDesignGetMesh
  (return (Variables|Default|GetItemMesh)))