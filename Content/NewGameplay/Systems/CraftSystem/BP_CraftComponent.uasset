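; BP_CraftComponent is an actor component that lets its owner craft items from DT_Craft recipes using the owner's inventory.
; On BeginPlay it caches the owner's BP_InventoryComponent.
; Craft looks up the recipe row, checks that every input is held in sufficient count, then removes the inputs and adds the output.
; Open and Close only toggle an IsOpen flag.
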(event EventBeginPlay
  (Variables|Default|SetOwnerInventory (Actor|GetComponentbyClass (Components|GetOwner) "/Game/NewGameplay/Systems/InventorySystem/BP_InventoryComponent.BP_InventoryComponent_C")))

(event EventTick
  (params (DeltaSeconds :type Float%20%28single-precision%29)))

(fn Craft
  (params (InCraft :type Name))
  (bind _returnvalue (Utilities|GetDataTableRow "/Game/NewGameplay/Systems/CraftSystem/DT_Craft.DT_Craft" InCraft)
    (:then
      (for _array_element (.Input (Utilities|Struct|BreakS_CraftTableData _returnvalue))
        (if (not (>= (Default|GetItemCount (Variables|Default|GetOwnerInventory) (.Item (Utilities|Struct|BreakS_CraftItemData _array_element))) (.Count (Utilities|Struct|BreakS_CraftItemData _array_element))))
          (return)))
      (for _array_element_2 (.Input (Utilities|Struct|BreakS_CraftTableData _returnvalue))
        (Default|RemoveItemCount (Variables|Default|GetOwnerInventory) (.Item (Utilities|Struct|BreakS_CraftItemData _array_element_2)) (.Count (Utilities|Struct|BreakS_CraftItemData _array_element_2))))
      (Default|AddItem (Variables|Default|GetOwnerInventory) (.Item (Utilities|Struct|BreakS_CraftItemData (.Output (Utilities|Struct|BreakS_CraftTableData _returnvalue)))) (.Count (Utilities|Struct|BreakS_CraftItemData (.Output (Utilities|Struct|BreakS_CraftTableData _returnvalue))))))))

(fn Open
  (Variables|Default|SetIsOpen true))

(fn Close
  (Variables|Default|SetIsOpen false))