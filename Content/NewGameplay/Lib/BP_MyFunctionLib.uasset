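; Blueprint function library that maps between the RPG-style attribute, stat, damage type and property-name identifiers used by gameplay code.
; Selects and switches convert attributes to regen and max prop names, link each stat to its attribute, and give damage and defense prop names per damage type.
; Reverse lookups read category, attribute, stat and damage type from DT_Props rows, with fallbacks for missing rows.
; A helper also returns an identity transform.
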(fn NullTransform
  (return (Math|Transform|MakeTransform "0, 0, 0")))

(fn ToRegenProp(Attribute)
  (params (Attribute :type EAttributeList%20Enum :default "EAL_None"))
  (return (Utilities|Select :Index Attribute :EAL_None "None" :EAL_Health "RegenHealth" :EAL_Mana "RegenMana" :EAL_Stamina "RegenStamina" :EAL_Air "RegenAir")))

(fn ToMaxProp(Attribute)
  (params (Attribute :type EAttributeList%20Enum :default "EAL_None"))
  (return (Utilities|Select :Index Attribute :EAL_None "None" :EAL_Health "MaxHealth" :EAL_Mana "MaxMana" :EAL_Stamina "MaxStamina" :EAL_Air "MaxAir")))

(fn GetStat(Attribute)
  (params (Attribute :type EAttributeList%20Enum :default "EAL_None"))
  (return (Utilities|Select :Index Attribute :EAL_None "ESL_None" :EAL_Health "ESL_Strength" :EAL_Mana "ESL_Intelligence" :EAL_Stamina "ESL_Dexterity" :EAL_Air "ESL_None")))

(fn GetCategory(Prop)
  (params (Prop :type Name))
  (bind _returnvalue (Utilities|GetDataTableRow "/Game/NewGameplay/Systems/PropSystem/DT_Props.DT_Props" Prop)
    (:then
      (return (Utilities|Struct|BreakGamePropertyTableData _returnvalue)))
    (:RowNotFound
      (return "EGPCL_None"))))

(fn GetAttribute(Prop)
  (params (Prop :type Name))
  (bind _returnvalue (Utilities|GetDataTableRow "/Game/NewGameplay/Systems/PropSystem/DT_Props.DT_Props" Prop)
    (:then
      (return (Utilities|Struct|BreakGamePropertyTableData _returnvalue)))
    (:RowNotFound
      (return "EAL_Health"))))

(fn GetStat(Prop)
  (params (Prop :type Name))
  (bind _returnvalue (Utilities|GetDataTableRow "/Game/NewGameplay/Systems/PropSystem/DT_Props.DT_Props" Prop)
    (:then
      (return (Utilities|Struct|BreakGamePropertyTableData _returnvalue)))
    (:RowNotFound
      (return "ESL_None"))))

(fn GetAttribute(Stat)
  (params (Stat :type EStatList%20Enum :default "ESL_None"))
  (return (Utilities|Select :Index Stat :ESL_None "EAL_None" :ESL_Strength "EAL_Health" :ESL_Dexterity "EAL_Stamina" :ESL_Intelligence "EAL_Mana")))

(fn GetDamageType(Prop)
  (params (Prop :type Name))
  (bind _returnvalue (Utilities|GetDataTableRow "/Game/NewGameplay/Systems/PropSystem/DT_Props.DT_Props" Prop)
    (:then
      (return (Utilities|Struct|BreakGamePropertyTableData _returnvalue)))
    (:RowNotFound
      (return "EDT_None"))))

(fn GetDamageProp(DamageType)
  (params (DamageType :type EDamageType%20Enum :default "EDT_None"))
  (switch Utilities|FlowControl|Switch|SwitchonEDamageType DamageType
    (:EDT_None
      (return "None"))
    (:EDT_Physical
      (return "DamagePhysical"))
    (:EDT_Cold
      (return "DamageCold"))
    (:EDT_Poison
      (return "DamagePoison"))
    (:EDT_Fire
      (return "DamageFire"))
    (:EDT_Electric
      (return "DamageElectric"))
    (:EDT_Magical
      (return "DamageMagical"))))

(fn GetDefenseProp(DamageType)
  (params (DamageType :type EDamageType%20Enum :default "EDT_None"))
  (switch Utilities|FlowControl|Switch|SwitchonEDamageType DamageType
    (:EDT_None
      (return "None"))
    (:EDT_Physical
      (return "DefensePhysical"))
    (:EDT_Cold
      (return "DefenseCold"))
    (:EDT_Poison
      (return "DefensePoison"))
    (:EDT_Fire
      (return "DefenseFire"))
    (:EDT_Electric
      (return "DefenseElectric"))
    (:EDT_Magical
      (return "DefenseMagical"))))

(fn GetStatProp(Stat)
  (params (Stat :type EStatList%20Enum :default "ESL_None"))
  (return (Utilities|Select :Index Stat :ESL_None "None" :ESL_Strength "Strength" :ESL_Dexterity "Dexterity" :ESL_Intelligence "Intelligence")))