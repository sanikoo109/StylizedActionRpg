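; Interactable torch holder that can start with a torch, takes one from either of the player's selected weapon slots, or returns it to their inventory.
; TorchItemSlot updates drive the mesh, cloth material and flame particles, with fire-change events bound to the held torch.
; A lit torch ignites actors entering FireSphere, Ignite lights the held torch, and AmbientLightComp is notified when the light state changes.
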(event OnComponentBeginOverlap(FireSphere)
  (params (OverlappedComponent :type Primitive%20Component%20Object%20Reference) (OtherActor :type Actor%20Object%20Reference) (OtherComp :type Primitive%20Component%20Object%20Reference) (OtherBodyIndex :type Integer) (bFromSweep :type Boolean) (SweepResult :type Hit%20Result%20Structure%20%28by%20ref%29))
  (bind _asii_torch (Utilities|Casting|CastToII_Torch (Variables|/Game/NewGameplay/Systems/InventorySystem/BP_InventoryItemSlot.BP_InventoryItemSlot_C|GetCurrentItem (Variables|Default|GetTorchItemSlot))))
  (if (Variables|/Game/NewGameplay/Items/II_Torch.II_Torch_C|GetbFire _asii_torch)
    (Class|BPTorchInterface|Ignite(Message) OtherActor)))

(event OnUpdateItem(TorchItemSlot)
  (params (NewItem :type Inventory%20Item%20Object%20Reference) (PrevItem :type Inventory%20Item%20Object%20Reference))
  (bind _asii_torch (Utilities|Casting|CastToII_Torch NewItem)
    (:then
      (Rendering|SetVisibility (Variables|Default|GetSM_Torch) true false)
      (if (Variables|/Game/NewGameplay/Items/II_Torch.II_Torch_C|GetbFire _asii_torch)
        (Rendering|Material|SetMaterial (Variables|Default|GetSM_Torch) 1 "/Game/NewGameplay/Materials/MI_MatInFire.MI_MatInFire")
        (Components|Activation|Activate (Variables|Default|GetP_TorchFire) false)
        (else
          (Rendering|Material|SetMaterial (Variables|Default|GetSM_Torch) 1 "/Game/NewGameplay/Materials/MI_Cloth_White.MI_Cloth_White")
          (Components|Activation|Deactivate (Variables|Default|GetP_TorchFire)))))
    (:CastFailed
      (Rendering|SetVisibility (Variables|Default|GetSM_Torch) false false))))

(event EventBeginPlay
  (EventDispatchers|AssignOnUpdateItem (Variables|Default|GetTorchItemSlot) (EventDispatchers|CreateEvent :!event OnUpdateItemEvent))
  (if (Variables|Default|GetbHaveTorch)
    (bind _returnvalue (Game|SpawnActorfromClass "/Game/NewGameplay/Items/II_Torch.II_Torch_C" (CallFunction|NullTransform) "Undefined" "MultiplyWithRoot" 0 (Variables|Default|GetbTorchFire) "Torch" 1 0))
    (Default|SetItem (Variables|Default|GetTorchItemSlot) _returnvalue)))

(event EventInteract
  (params (Char :type Character%20Object%20Reference) (TargetComp :type Primitive%20Component%20Object%20Reference))
  (bind _asbp_my_character (Utilities|Casting|CastToBP_MyCharacter Char))
  (CallFunction|InteractFunc _asbp_my_character))

(event EventIgnite
  (bind _asii_torch (Utilities|Casting|CastToII_Torch (Variables|/Game/NewGameplay/Systems/InventorySystem/BP_InventoryItemSlot.BP_InventoryItemSlot_C|GetCurrentItem (Variables|Default|GetTorchItemSlot))))
  (Default|SetFire _asii_torch true))

(fn ConstructionScript)

(fn OnUpdateItemEvent
  (params (NewItem :type Inventory%20Item%20Object%20Reference) (PrevItem :type Inventory%20Item%20Object%20Reference))
  (Utilities|FlowControl|Sequence
    (:then_0
      (bind _asii_torch (Utilities|Casting|CastToII_Torch PrevItem))
      (EventDispatchers|UnbindEventfromOnFireUpdate _asii_torch (EventDispatchers|CreateEvent :!event TorchFireUpdate))
      (LocalVariables|SetLocal_PrevFire (Variables|/Game/NewGameplay/Items/II_Torch.II_Torch_C|GetbFire _asii_torch)))
    (:then_1
      (bind _asii_torch_2 (Utilities|Casting|CastToII_Torch NewItem))
      (EventDispatchers|BindEventtoOnFireUpdate _asii_torch_2 (EventDispatchers|CreateEvent :!event TorchFireUpdate))
      (LocalVariables|SetLocal_NewFire (Variables|/Game/NewGameplay/Items/II_Torch.II_Torch_C|GetbFire _asii_torch_2)))
    (:then_2
      (if (!= (LocalVariables|GetLocal_PrevFire) (LocalVariables|GetLocal_NewFire))
        (Default|NotifySourceUpdate (Variables|Default|GetAmbientLightComp))))))

(fn TorchFireUpdate
  (params (IsActive :type Boolean))
  (Utilities|FlowControl|Sequence
    (:then_0
      (Default|NotifySourceUpdate (Variables|Default|GetAmbientLightComp)))
    (:then_1
      (if IsActive
        (Components|Activation|Activate (Variables|Default|GetP_TorchFire) false)
        (Rendering|Material|SetMaterial (Variables|Default|GetSM_Torch) 1 "/Game/NewGameplay/Materials/MI_MatInFire.MI_MatInFire")
        (else
          (Components|Activation|Deactivate (Variables|Default|GetP_TorchFire))
          (Rendering|Material|SetMaterial (Variables|Default|GetSM_Torch) 1 "/Game/NewGameplay/Materials/MI_Cloth_White.MI_Cloth_White"))))))

(fn InteractFunc
  (params (Char :type BP%20My%20Character%20Object%20Reference))
  (bind _inventorycomponent (Variables|/Game/NewGameplay/Characters/BP_MyCharacter.BP_MyCharacter_C|GetInventoryComponent Char))
  (if (Default|IsEmpty (Variables|Default|GetTorchItemSlot))
    (Utilities|FlowControl|Sequence
      (:then_0
        (LocalVariables|SetLocal_Item (Default|GetSelectedSlotItem _inventorycomponent "EIST_WeaponL")))
      (:then_1
        (LocalVariables|SetLocal_Item (Default|GetSelectedSlotItem _inventorycomponent "EIST_WeaponR"))))
    (bind _local_item (LocalVariables|GetLocal_Item)
      (:then
        (if (== (Variables|/Game/NewGameplay/Systems/InventorySystem/BP_InventoryItem.BP_InventoryItem_C|GetItemRowName _local_item) "Torch")
          (Default|RemovefromParent (LocalVariables|GetLocal_Item))
          (Default|SetItem (Variables|Default|GetTorchItemSlot) (LocalVariables|GetLocal_Item))
          (return)))
      (:else))
    (else
      (bind _returnvalue (Default|AddItemRef _inventorycomponent (Variables|/Game/NewGameplay/Systems/InventorySystem/BP_InventoryItemSlot.BP_InventoryItemSlot_C|GetCurrentItem (Variables|Default|GetTorchItemSlot))))
      (if _returnvalue
        (Default|SetItem (Variables|Default|GetTorchItemSlot))))))

(fn GetInteractInfo
  (params (Char :type Character%20Object%20Reference) (TargetComp :type Primitive%20Component%20Object%20Reference))
  (return (Utilities|Struct|MakeInteractInfo "EIT_Default" "Torch")))

(fn IsLightSourceActive
  (bind _asii_torch (Utilities|Casting|CastToII_Torch (Variables|/Game/NewGameplay/Systems/InventorySystem/BP_InventoryItemSlot.BP_InventoryItemSlot_C|GetCurrentItem (Variables|Default|GetTorchItemSlot)))
    (:then
      (return (Variables|/Game/NewGameplay/Items/II_Torch.II_Torch_C|GetbFire _asii_torch)))
    (:CastFailed
      (return false))))