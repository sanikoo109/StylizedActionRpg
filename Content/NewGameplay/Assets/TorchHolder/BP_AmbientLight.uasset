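; BP_AmbientLight is an ambient point light whose intensity depends on how many of its linked light sources, such as torch holders, are active.
; On BeginPlay it sets the initial intensity and binds to the OnUpdateSource dispatcher on each source's BP_AmbientLightSourceComp.
; Each update counts active sources through IsLightSourceActiveMessage and uses that count as an index into IntensityList to set the PointLightComponent's intensity.
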(event Custom|OnUpdateSource_Event
  (CallFunction|UpdateLightIntensity))

(event EventBeginPlay
  (CallFunction|UpdateLightIntensity)
  (for _array_element (Variables|Default|GetLightSources)
    (EventDispatchers|AssignOnUpdateSource (Actor|GetComponentbyClass _array_element "/Game/NewGameplay/Assets/TorchHolder/BP_AmbientLightSourceComp.BP_AmbientLightSourceComp_C") (delegate Custom|OnUpdateSource_Event))))

(fn ConstructionScript)

(fn UpdateLightIntensity
  (for _array_element (Variables|Default|GetLightSources)
    (bind _result (Class|BPAmbientLightInterface|IsLightSourceActive(Message) _array_element))
    (if _result
      (Math|Integer|IncrementInt (LocalVariables|GetActiveSources))))
  (Rendering|Components|Light|SetIntensity (Variables|Default|GetPointLightComponent) (Utilities|Array|Get(acopy) (Variables|Default|GetIntensityList) (LocalVariables|GetActiveSources))))