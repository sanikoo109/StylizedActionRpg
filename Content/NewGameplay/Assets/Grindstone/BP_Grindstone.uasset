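; BP_Grindstone is an interactable grindstone that offers a "Sharpen weapon" prompt.
; On Interact, it gets the character's inventory component and applies the "SharpWeapon" buff through the BuffComponent of each valid selected right and left weapon slot item.
; It then activates its particle system, whether or not a weapon was found.
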(event EventBeginPlay)

(event Collision|EventActorBeginOverlap
  (params (OtherActor :type Actor%20Object%20Reference)))

(event EventTick
  (params (DeltaSeconds :type Float%20%28single-precision%29)))

(event EventInteract
  (params (Char :type Character%20Object%20Reference) (TargetComp :type Primitive%20Component%20Object%20Reference))
  (bind _returnvalue (Actor|GetComponentbyClass Char "/Game/NewGameplay/Systems/InventorySystem/BP_InventoryComponent.BP_InventoryComponent_C"))
  (bind _returnvalue_2 (Default|GetSelectedSlotItem _returnvalue "EIST_WeaponL"))
  (bind _returnvalue_3 (Default|GetSelectedSlotItem _returnvalue "EIST_WeaponR"))
  (Utilities|FlowControl|Sequence
    (:then_0
      (Utilities|IsValid _returnvalue_3
        (:Is%20Valid
          (Default|PlayBuff (Variables|/Game/NewGameplay/Systems/InventorySystem/BP_InventoryItem.BP_InventoryItem_C|GetBuffComponent _returnvalue_3) "SharpWeapon"))))
    (:then_1
      (Utilities|IsValid _returnvalue_2
        (:Is%20Valid
          (Default|PlayBuff (Variables|/Game/NewGameplay/Systems/InventorySystem/BP_InventoryItem.BP_InventoryItem_C|GetBuffComponent _returnvalue_2) "SharpWeapon"))))
    (:then_2
      (Components|Activation|Activate (Variables|Default|GetParticleSystem) true))))

(fn ConstructionScript)

(fn GetInteractInfo
  (params (Char :type Character%20Object%20Reference) (TargetComp :type Primitive%20Component%20Object%20Reference))
  (return (Utilities|Struct|MakeInteractInfo "EIT_Default" "Sharpen weapon")))