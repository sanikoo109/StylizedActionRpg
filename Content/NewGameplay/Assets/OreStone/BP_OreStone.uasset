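; BP_OreStone is a mineable ore rock whose ore type sets its material in the construction script.
; On BeginPlay it spawns an inventory item of that ore and count into its InventoryItemSlot.
; Point damage from a Pickaxe item splits off one unit into the instigator's inventory and spawns sparks at the hit.
; When the slot's item becomes invalid, the ore material switches to dark stone.
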(event OnUpdateItem(InventoryItemSlot)
  (params (NewItem :type Inventory%20Item%20Object%20Reference) (PrevItem :type Inventory%20Item%20Object%20Reference))
  (Utilities|IsValid NewItem
    (:Is%20Not%20Valid
      (Rendering|Material|SetMaterial (Variables|Default|GetSM_OreStone) 1 "/Game/NewGameplay/Materials/MI_Stone_Dark.MI_Stone_Dark"))))

(event EventBeginPlay
  (bind _returnvalue (Game|SpawnActorfromClass "/Game/NewGameplay/Systems/InventorySystem/BP_InventoryItem.BP_InventoryItem_C" (CallFunction|NullTransform) "Undefined" "MultiplyWithRoot" 0 (CallFunction|GetOreItemName (Variables|Default|GetOre)) (Variables|Default|GetCount) 0))
  (Default|SetItem (Variables|Default|GetInventoryItemSlot) _returnvalue))

(event Collision|EventActorBeginOverlap
  (params (OtherActor :type Actor%20Object%20Reference)))

(event EventTick
  (params (DeltaSeconds :type Float%20%28single-precision%29)))

(event Game|Damage|EventPointDamage
  (params (Damage :type Float%20%28single-precision%29) (DamageType :type Damage%20Type%20Object%20Reference) (HitLocation :type Vector :default "0, 0, 0") (HitNormal :type Vector :default "0, 0, 0") (HitComponent :type Primitive%20Component%20Object%20Reference) (BoneName :type Name :default "None") (ShotFromDirection :type Vector :default "0, 0, 0") (InstigatedBy :type Controller%20Object%20Reference) (DamageCauser :type Actor%20Object%20Reference) (HitInfo :type Hit%20Result%20Structure%20%28by%20ref%29))
  (bind _returnvalue (Actor|GetComponentbyClass DamageCauser "/Game/NewGameplay/Systems/InventorySystem/BP_DesignItemLogicComp.BP_DesignItemLogicComp_C"))
  (Utilities|IsValid DamageCauser
    (:Is%20Valid
      (Utilities|IsValid _returnvalue
        (:Is%20Valid
          (bind _parentitem (Variables|/Game/NewGameplay/Systems/InventorySystem/BP_DesignItemLogicComp.BP_DesignItemLogicComp_C|GetParentItem _returnvalue)
            (:then
              (if (== (Variables|/Game/NewGameplay/Systems/InventorySystem/BP_InventoryItem.BP_InventoryItem_C|GetItemRowName _parentitem) "Pickaxe")
                (bind _currentitem (Variables|/Game/NewGameplay/Systems/InventorySystem/BP_InventoryItemSlot.BP_InventoryItemSlot_C|GetCurrentItem (Variables|Default|GetInventoryItemSlot))
                  (:then
                    (bind _returnvalue_2 (Default|Split _currentitem 1))
                    (Default|AddItemRef (Actor|GetComponentbyClass (Pawn|GetControlledPawn InstigatedBy) "/Game/NewGameplay/Systems/InventorySystem/BP_InventoryComponent.BP_InventoryComponent_C") _returnvalue_2)
                    (Effects|SpawnEmitteratLocation "/Game/NewGameplay/Effects/P_BlockSparks.P_BlockSparks" HitLocation))
                  (:else))))
            (:else)))))))

(fn ConstructionScript
  (Rendering|Material|SetMaterial (Variables|Default|GetSM_OreStone) 1 (Utilities|Select :Index (Variables|Default|GetOre) :NewEnumerator0 "/Game/NewGameplay/Materials/MI_Black.MI_Black" :NewEnumerator1 "/Game/NewGameplay/Materials/MI_Steel_Black.MI_Steel_Black" :NewEnumerator2 "/Game/NewGameplay/Materials/MI_Silver_Rough.MI_Silver_Rough" :NewEnumerator3 "/Game/NewGameplay/Materials/MI_Gold_Rough.MI_Gold_Rough" :NewEnumerator4 "/Game/NewGameplay/Materials/MI_Platinum_Rough.MI_Platinum_Rough")))

(fn GetOreItemName
  (params (Ore :type E_OreList%20Enum :default "NewEnumerator0"))
  (return (Utilities|Select :Index Ore :NewEnumerator0 "None" :NewEnumerator1 "IronOre" :NewEnumerator2 "SilverOre" :NewEnumerator3 "GoldOre" :NewEnumerator4 "PlatinumOre")))