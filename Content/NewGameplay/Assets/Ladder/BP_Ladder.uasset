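; BP_Ladder is a climbable ladder actor that starts the ladder move on a BP_MyCharacter touching its box trigger.
; On overlap it converts the character's foot height into the nearest step index and passes it, with itself, to BPParkourComponent's BeginLadder.
; The construction script sizes and centers the trigger from width, step count and step height, then draws temporary debug boxes to preview each rung.
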(event OnComponentBeginOverlap(Box)
  (params (OverlappedComponent :type Primitive%20Component%20Object%20Reference) (OtherActor :type Actor%20Object%20Reference) (OtherComp :type Primitive%20Component%20Object%20Reference) (OtherBodyIndex :type Integer) (bFromSweep :type Boolean) (SweepResult :type Hit%20Result%20Structure%20%28by%20ref%29))
  (bind _asbp_my_character (Utilities|Casting|CastToBP_MyCharacter OtherActor))
  (Class|ParkourComponent|BeginLadder (Variables|/Game/NewGameplay/Characters/BP_MyCharacter.BP_MyCharacter_C|GetBP_ParkourComponent _asbp_my_character) self (Math|Float|Round (/ (.z (- (- (Transformation|GetActorLocation _asbp_my_character) (Math|Vector|MakeVector 0.0 0.0 (Components|Capsule|GetScaledCapsuleHalfHeight (Variables|/Script/Engine.Character|GetCapsuleComponent _asbp_my_character)))) (Transformation|GetActorLocation))) (Variables|Default|GetStepHeight)))))

(event EventBeginPlay)

(event Collision|EventActorBeginOverlap
  (params (OtherActor :type Actor%20Object%20Reference)))

(event EventTick
  (params (DeltaSeconds :type Float%20%28single-precision%29)))

(fn ConstructionScript
  (bind _stepheight (Variables|Default|GetStepHeight))
  (Variables|Ladder|SetbUpdateDebugDraw false)
  (Utilities|FlowControl|Sequence
    (:then_0
      (Components|Box|SetBoxExtent (Variables|Default|GetBox) (Math|Vector|MakeVector 25.0 (+ (/ (Variables|Default|GetWidth) 2.0) 1e+01) (+ (/ (* (- (Variables|Default|GetStepCount) 1) (Variables|Default|GetStepHeight)) 2.0) 1e+01)) true)
      (Transformation|SetRelativeLocation (Variables|Default|GetBox) (Math|Vector|MakeVector 0.0 0.0 (/ (- (* (Variables|Default|GetStepCount) _stepheight) _stepheight) 2.0)) false false))
    (:then_1
      (Rendering|Debug|FlushPersistentDebugLines)
      (for _index (range 0 (- (Variables|Default|GetStepCount) 1))
        (Rendering|Debug|DrawDebugBox (.location (Math|Transform|ComposeTransforms (Math|Transform|MakeTransform (Math|Vector|MakeVector 0.0 0.0 (* _index (Variables|Default|GetStepHeight))) "0, 0, 0" "1.000000,1.000000,1.000000") (Transformation|GetActorTransform))) (Math|Vector|MakeVector 5.0 (/ (Variables|Default|GetWidth) 2.0) 5.0) "(R=0.000000,G=1.000000,B=0.058253,A=1.000000)" (.rotation (Math|Transform|ComposeTransforms (Math|Transform|MakeTransform (Math|Vector|MakeVector 0.0 0.0 (* _index (Variables|Default|GetStepHeight))) "0, 0, 0" "1.000000,1.000000,1.000000") (Transformation|GetActorTransform))) 25.0 0.0)))))