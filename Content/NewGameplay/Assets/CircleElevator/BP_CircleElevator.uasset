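; BP_CircleElevator is a circular elevator that moves between its base position and a configurable Height vector when BP_MyCharacter enters its trigger boxes.
; A timeline lerps the mesh's relative location, playing to rise and reversing to descend.
; Box toggles direction, while Box_Up and Box_Down force one; MoveUp and MoveDown ignore calls while the timeline plays.
; The construction script places BoxUp slightly above the Height offset.
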(event OnComponentBeginOverlap(Box)
  (params (OverlappedComponent :type Primitive%20Component%20Object%20Reference) (OtherActor :type Actor%20Object%20Reference) (OtherComp :type Primitive%20Component%20Object%20Reference) (OtherBodyIndex :type Integer) (bFromSweep :type Boolean) (SweepResult :type Hit%20Result%20Structure%20%28by%20ref%29))
  (Utilities|Casting|CastToBP_MyCharacter OtherActor)
  (CallFunction|Move))

(event OnComponentBeginOverlap(Box_Up)
  (params (OverlappedComponent :type Primitive%20Component%20Object%20Reference) (OtherActor :type Actor%20Object%20Reference) (OtherComp :type Primitive%20Component%20Object%20Reference) (OtherBodyIndex :type Integer) (bFromSweep :type Boolean) (SweepResult :type Hit%20Result%20Structure%20%28by%20ref%29))
  (Utilities|Casting|CastToBP_MyCharacter OtherActor)
  (CallFunction|MoveUp))

(event OnComponentBeginOverlap(Box_Down)
  (params (OverlappedComponent :type Primitive%20Component%20Object%20Reference) (OtherActor :type Actor%20Object%20Reference) (OtherComp :type Primitive%20Component%20Object%20Reference) (OtherBodyIndex :type Integer) (bFromSweep :type Boolean) (SweepResult :type Hit%20Result%20Structure%20%28by%20ref%29))
  (Utilities|Casting|CastToBP_MyCharacter OtherActor)
  (CallFunction|MoveDown))

(event Custom|Move
  (if (Variables|Default|GetbUp)
    (CallFunction|MoveDown)
    (else
      (CallFunction|MoveUp))))

(event Custom|MoveUp
  (if (not (Audio|Components|Audio|IsPlaying (Variables|Default|GetElevatorTimeline)))
    (Variables|Default|SetbUp true)
    (bind _driver (Timeline|ElevatorTimeline Play)
      (:Update
        (Transformation|SetRelativeLocation (Variables|Default|GetSM_CircleElevator) (Math|Vector|Lerp(Vector) "0, 0, 0" (Variables|Default|GetHeight) _driver) false false)))))

(event Custom|MoveDown
  (if (not (Audio|Components|Audio|IsPlaying (Variables|Default|GetElevatorTimeline)))
    (Variables|Default|SetbUp false)
    (bind _driver (Timeline|ElevatorTimeline Reverse)
      (:Update
        (Transformation|SetRelativeLocation (Variables|Default|GetSM_CircleElevator) (Math|Vector|Lerp(Vector) "0, 0, 0" (Variables|Default|GetHeight) _driver) false false)))))

(event EventBeginPlay)

(event Collision|EventActorBeginOverlap
  (params (OtherActor :type Actor%20Object%20Reference)))

(event EventTick
  (params (DeltaSeconds :type Float%20%28single-precision%29)))

(fn ConstructionScript
  (Transformation|SetRelativeLocation (Variables|Default|GetBox_Up) (+ (Variables|Default|GetHeight) "0.000000,0.000000,150.000000") false false))