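; BP_Corpse is a lootable corpse actor that shows a "Loot" interaction prompt.
; Its construction script copies the exposed Items list into its inventory component's start items and sets the skeletal mesh's animation from the Anim variable.
; Interacting calls InspectInventory on the interacting character's BP_InventoryComponent, passing the corpse's own inventory.
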(event EventBeginPlay)

(event Collision|EventActorBeginOverlap
  (params (OtherActor :type Actor%20Object%20Reference)))

(event EventTick
  (params (DeltaSeconds :type Float%20%28single-precision%29)))

(event EventInteract
  (params (Char :type Character%20Object%20Reference) (TargetComp :type Primitive%20Component%20Object%20Reference))
  (Default|InspectInventory (Actor|GetComponentbyClass Char "/Game/NewGameplay/Systems/InventorySystem/BP_InventoryComponent.BP_InventoryComponent_C") (Variables|Default|GetInventoryComponent)))

(fn ConstructionScript
  (Variables|/Game/NewGameplay/Systems/InventorySystem/BP_InventoryComponent.BP_InventoryComponent_C|SetStartItems (Variables|Default|GetInventoryComponent) (Variables|Default|GetItems))
  (Utilities|Struct|SetmembersinSingleAnimationPlayData (Variables|/Script/Engine.SkeletalMeshComponent|GetAnimationData (Variables|Default|GetSkeletalMesh)) (Variables|Default|GetAnim)))

(fn GetInteractInfo
  (params (Char :type Character%20Object%20Reference) (TargetComp :type Primitive%20Component%20Object%20Reference))
  (return (Utilities|Struct|MakeInteractInfo "EIT_Default" "Loot")))