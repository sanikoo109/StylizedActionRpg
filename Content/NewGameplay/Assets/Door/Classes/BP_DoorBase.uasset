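; Base interactable door that opens on a timeline, with rotation left for child Blueprints to implement.
; It can be key-locked through the character's inventory or latched by an animated locker that releases only from inside.
; Open and locker changes fire update events that drive the timelines.
; A smart nav link, disabled while locked, aligns arriving characters and opens the door, and overlapping enemies prevent closing.
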(event OnComponentBeginOverlap(Box)
  (params (OverlappedComponent :type Primitive%20Component%20Object%20Reference) (OtherActor :type Actor%20Object%20Reference) (OtherComp :type Primitive%20Component%20Object%20Reference) (OtherBodyIndex :type Integer) (bFromSweep :type Boolean) (SweepResult :type Hit%20Result%20Structure%20%28by%20ref%29)))

(event OnComponentEndOverlap(Box)
  (params (OverlappedComponent :type Primitive%20Component%20Object%20Reference) (OtherActor :type Actor%20Object%20Reference) (OtherComp :type Primitive%20Component%20Object%20Reference) (OtherBodyIndex :type Integer)))

(event Custom|OpenWithDelay
  (Utilities|FlowControl|Delay 0.3)
  (CallFunction|SetOpen true))

(event Custom|OnSmartLinkReached_Event
  (params (MovingActor :type Actor%20Object%20Reference) (DestinationPoint :type Vector%20%28by%20ref%29))
  (bind _asbp_my_character (Utilities|Casting|CastToBP_MyCharacter MovingActor))
  (Default|Align _asbp_my_character (Math|Transform|ComposeTransforms (Math|Transform|MakeTransform (Math|Vector|MakeVector 0.0 0.0 (Components|Capsule|GetScaledCapsuleHalfHeight (Variables|/Script/Engine.Character|GetCapsuleComponent _asbp_my_character))) "0, 0, 0" "1.000000,1.000000,1.000000") (Transformation|GetWorldTransform (select (CallFunction|IsInsideDoor MovingActor) (Variables|Default|GetCharInsidePoint) (Variables|Default|GetCharOutsidePoint)))) 0.5)
  (CallFunction|SetOpen true))

(event Custom|TryCharOpenDoor
  (params (Char :type BP%20My%20Character%20Object%20Reference))
  (if (Variables|Default|GetCanOpenByAI)
    (if (CallFunction|IsOverlappingAnyEnemy)
      (if (not (Variables|Default|GetIsOpen))
        (Utilities|FlowControl|Sequence
          (:then_0
            (CallFunction|SetOpen true))
          (:then_2
            (for _array_element (Collision|GetOverlappingActors (Variables|Default|GetBox) "/Game/NewGameplay/Characters/BP_MyCharacter.BP_MyCharacter_C" :!class /Script/Engine.PrimitiveComponent)
              (bind _asaic_enemy (Utilities|Casting|CastToAIC_Enemy (AI|GetAIController _array_element)))
              (Default|StopMoveAlongTime _asaic_enemy (* (Variables|Default|GetOpenTime) (- 1.0 (Components|Timeline|GetPlaybackPosition (Variables|Default|GetOpenTimeline))))))))))))

(event Custom|UpdateInstantRotation
  (params (Rotation :type Float%20%28double-precision%29)))

(event Custom|OnLockerUpdate_Event
  (params (IsLocked :type Boolean))
  (CallFunction|UpdateNavLink)
  (if IsLocked
    (bind _driver (Timeline|LockerTimeline Play)
      (:Update
        (Transformation|SetRelativeLocation (Variables|Default|GetSM_Locker_Locker_Move) (Math|Vector|Lerp(Vector) "0, 0, 0" "0.000000,-10.000000,0.000000" _driver) false false)))
    (else
      (Timeline|LockerTimeline Reverse))))

(event Custom|UpdateDoorRotation
  (params (Rotation :type Float%20%28double-precision%29)))

(event Custom|UpdateNavLink
  (bind _navlink (Variables|Default|GetNavLink)
    (:then
      (Class|NavLinkProxy|SetSmartLinkEnabled _navlink (not (or (Variables|Default|GetbKeyLocked) (Variables|Default|GetbLockerLocked)))))
    (:else)))

(event Custom|OnOpenUpdate_Event
  (params (bOpen :type Boolean))
  (CallFunction|UpdateInstantRotation (Math|Float|SelectFloat (Variables|Default|GetMaxAngle) 0.0 (Variables|Default|GetIsOpen)))
  (if bOpen
    (bind _driver (Timeline|OpenTimeline Play)
      (:Update
        (CallFunction|UpdateDoorRotation (Math|Float|Lerp 0.0 (Variables|Default|GetMaxAngle) _driver))))
    (else
      (Timeline|OpenTimeline Reverse))))

(event EventBeginPlay
  (EventDispatchers|BindEventtoOnOpenUpdate (EventDispatchers|CreateEvent :!event Custom|OnOpenUpdate_Event))
  (EventDispatchers|BindEventtoOnLockerUpdate (EventDispatchers|CreateEvent :!event Custom|OnLockerUpdate_Event))
  (Components|Timeline|SetPlayRate (Variables|Default|GetOpenTimeline) (/ 1.0 (Variables|Default|GetOpenTime)))
  (CallFunction|UpdateNavLink)
  (Utilities|FlowControl|Sequence
    (:then_0
      (bind _returnvalue (Utilities|GetDataTableRow "/Game/NewGameplay/Systems/InventorySystem/Data/DTC_Items.DTC_Items" (Variables|Default|GetNeededKey))
        (:then
          (Variables|Default|SetKeyTableData _returnvalue))))
    (:then_1
      (bind _navlink (Variables|Default|GetNavLink)
        (:then
          (EventDispatchers|AssignOnSmartLinkReached _navlink (delegate Custom|OnSmartLinkReached_Event)))
        (:else)))))

(event EventInteract
  (params (Char :type Character%20Object%20Reference) (TargetComp :type Primitive%20Component%20Object%20Reference))
  (bind _asbp_my_character (Utilities|Casting|CastToBP_MyCharacter Char))
  (CallFunction|InteractFunction _asbp_my_character))

(fn ConstructionScript
  (Components|Timeline|SetPlaybackPosition (Variables|Default|GetOpenTimeline) (Math|Float|SelectFloat (Components|Timeline|GetTimelineLength (Variables|Default|GetOpenTimeline)) 0.0 (Variables|Default|GetIsOpen)) false true)
  (CallFunction|UpdateInstantRotation (Math|Float|SelectFloat (Variables|Default|GetMaxAngle) 0.0 (Variables|Default|GetIsOpen)))
  (Rendering|SetVisibility (Variables|Default|GetSM_Locker_Locker) (Variables|Default|GetbHaveLocker) true)
  (Components|Timeline|SetPlaybackPosition (Variables|Default|GetLockerTimeline) (Math|Float|SelectFloat (Components|Timeline|GetTimelineLength (Variables|Default|GetLockerTimeline)) 0.0 (Variables|Default|GetbLockerLocked)) false true))

(fn GetDoorMeshes
  (return 0))

(fn SetOpen
  (params (bOpen :type Boolean))
  (if (and (not (Variables|Default|GetbLockerLocked)) (not (Variables|Default|GetbKeyLocked)))
    (if (!= bOpen (Variables|Default|GetIsOpen))
      (bind _output_get (Variables|Default|SetIsOpen bOpen))
      (Default|CallOnOpenUpdate _output_get))))

(fn IsInsideDoor
  (params (Actor :type Actor%20Object%20Reference))
  (return (>= (Math|Vector|DotProduct (Math|Vector|Normalize (- (Transformation|GetActorLocation Actor) (Transformation|GetWorldLocation (Variables|Default|GetForwardDirection)))) (Math|Vector|GetForwardVector (Variables|Default|GetForwardDirection))) 0.0)))

(fn IsOverlappingAnyEnemy
  (return (> (- (Utilities|Array|Length (Collision|GetOverlappingActors (Variables|Default|GetBox) "/Game/NewGameplay/Characters/BP_MyCharacter.BP_MyCharacter_C" :!class /Script/Engine.PrimitiveComponent)) (Utilities|Array|Length (Collision|GetOverlappingActors (Variables|Default|GetBox) "/Game/NewGameplay/Characters/Player/Char_Player.Char_Player_C" :!class /Script/Engine.PrimitiveComponent))) 0)))

(fn SetLocker
  (params (IsLocked :type Boolean))
  (if (!= IsLocked (Variables|Default|GetbLockerLocked))
    (bind _output_get (Variables|Default|SetbLockerLocked IsLocked))
    (Default|CallOnLockerUpdate _output_get)))

(fn InteractFunction
  (params (Char :type BP%20My%20Character%20Object%20Reference))
  (if (Variables|Default|GetIsOpen)
    (if (not (CallFunction|IsOverlappingAnyEnemy))
      (CallFunction|SetOpen false))
    (else
      (Utilities|FlowControl|Sequence
        (:then_0
          (if (Variables|Default|GetbLockerLocked)
            (if (CallFunction|IsInsideDoor Char)
              (CallFunction|SetLocker false)
              (LocalVariables|SetLocal_bNeedDelay true)
              (else
                (return)))))
        (:then_1
          (if (Variables|Default|GetbKeyLocked)
            (if (Default|HaveItem (Variables|/Game/NewGameplay/Characters/BP_MyCharacter.BP_MyCharacter_C|GetInventoryComponent Char) (Variables|Default|GetNeededKey))
              (Variables|Default|SetbKeyLocked false)
              (CallFunction|UpdateNavLink)
              (LocalVariables|SetLocal_bNeedDelay true)
              (if (Variables|Default|GetbRemoveKey)
                (Default|RemoveItemCount (Variables|/Game/NewGameplay/Characters/BP_MyCharacter.BP_MyCharacter_C|GetInventoryComponent Char) (Variables|Default|GetNeededKey) 1))
              (else
                (return)))))
        (:then_2
          (if (LocalVariables|GetLocal_bNeedDelay)
            (CallFunction|OpenwithDelay)
            (else
              (CallFunction|SetOpen true))))))))

(fn GetInteractInfo
  (params (Char :type Character%20Object%20Reference) (TargetComp :type Primitive%20Component%20Object%20Reference))
  (if (Variables|Default|GetbKeyLocked)
    (bind _output_get (LocalVariables|SetLocal_InventoryComp (Actor|GetComponentbyClass Char "/Game/NewGameplay/Systems/InventorySystem/BP_InventoryComponent.BP_InventoryComponent_C")))
    (if (Default|HaveItem _output_get (Variables|Default|GetNeededKey))
      (return (Utilities|Struct|MakeInteractInfo "EIT_Default" (Utilities|Text|FormatText "Unlock using: {KeyName}" (Utilities|Struct|BreakInventoryItemTableData (Variables|Default|GetKeyTableData)))))
      (else
        (return (Utilities|Struct|MakeInteractInfo "EIT_Fail" (Utilities|Text|FormatText "Needed: {KeyName}" (Utilities|Struct|BreakInventoryItemTableData (Variables|Default|GetKeyTableData)))))))
    (else
      (if (Variables|Default|GetbLockerLocked)
        (if (CallFunction|IsInsideDoor Char)
          _
          (else
            (return (Utilities|Struct|MakeInteractInfo "EIT_Fail" "Locker from other side")))))
      (return (Utilities|Struct|MakeInteractInfo "EIT_Default" (select (Variables|Default|GetIsOpen) "Close" "Open"))))))