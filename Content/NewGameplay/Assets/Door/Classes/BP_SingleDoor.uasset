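; BP_SingleDoor is a single-leaf door that extends a parent door class through overridden events and functions.
; Its construction script attaches the door mesh and an instant-rotation pivot to the frame's Door socket, and the locker mesh to the door's Locker socket.
; Two rotation events apply negated yaw to the door and pivot separately, and GetDoorMeshes returns the one mesh.
; An old routine that pushes overlapping characters remains unconnected.
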(event EventUpdateInstantRotation
  (params (Rotation :type Float%20%28double-precision%29))
  (Transformation|SetRelativeRotation (Variables|Default|GetInstantRotationPivot) (Math|Rotator|MakeRotator 0.0 0.0 (* Rotation -1.0)) false false))

(event EventUpdateDoorRotation
  (params (Rotation :type Float%20%28double-precision%29))
  (Transformation|SetRelativeRotation (Variables|Default|GetDoor) (Math|Rotator|MakeRotator 0.0 0.0 (* Rotation -1.0)) false false))

(fn ConstructionScript
  (|CallParentFunction)
  (Transformation|AttachComponentToComponent (Variables|Default|GetDoor) (Variables|Default|GetFrame) "Door" "KeepRelative" "KeepRelative" "KeepRelative" true)
  (Transformation|AttachComponentToComponent (Variables|Default|GetInstantRotationPivot) (Variables|Default|GetFrame) "Door" "KeepRelative" "KeepRelative" "KeepRelative" true)
  (Transformation|AttachComponentToComponent (Variables|Default|GetSM_Locker_Locker) (Variables|Default|GetDoor) "Locker" "KeepRelative" "KeepRelative" "KeepRelative" true))

(fn GetDoorMeshes
  (return (Utilities|Array|MakeArray (Variables|Default|GetDoor))))