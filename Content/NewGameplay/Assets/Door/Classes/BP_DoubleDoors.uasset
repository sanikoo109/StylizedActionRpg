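; Double-door variant of a parent door Blueprint, with two leaves that swing in mirror image.
; The construction script attaches both doors and their instant-rotation pivots to the DoorR and DoorL sockets on the Frame.
; Rotation update events apply yaw to the right side and its negation to the left, separately for doors and pivots.
; GetDoorMeshes returns both leaves.
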(event EventUpdateInstantRotation
  (params (Rotation :type Float%20%28double-precision%29))
  (Transformation|SetRelativeRotation (Variables|Default|GetInstantRotationPivot_R) (Math|Rotator|MakeRotator 0.0 0.0 Rotation) false false)
  (Transformation|SetRelativeRotation (Variables|Default|GetInstantRotationPivot_L) (Math|Rotator|MakeRotator 0.0 0.0 (* Rotation -1.0)) false false))

(event EventUpdateDoorRotation
  (params (Rotation :type Float%20%28double-precision%29))
  (Transformation|SetRelativeRotation (Variables|Default|GetDoorR) (Math|Rotator|MakeRotator 0.0 0.0 Rotation) false false)
  (Transformation|SetRelativeRotation (Variables|Default|GetDoorL) (Math|Rotator|MakeRotator 0.0 0.0 (* Rotation -1.0)) false false))

(fn ConstructionScript
  (|CallParentFunction)
  (Transformation|AttachComponentToComponent (Variables|Default|GetDoorR) (Variables|Default|GetFrame) "DoorR" "KeepRelative" "KeepRelative" "KeepRelative" true)
  (Transformation|AttachComponentToComponent (Variables|Default|GetInstantRotationPivot_R) (Variables|Default|GetFrame) "DoorR" "KeepRelative" "KeepRelative" "KeepRelative" true)
  (Transformation|AttachComponentToComponent (Variables|Default|GetDoorL) (Variables|Default|GetFrame) "DoorL" "KeepRelative" "KeepRelative" "KeepRelative" true)
  (Transformation|AttachComponentToComponent (Variables|Default|GetInstantRotationPivot_L) (Variables|Default|GetFrame) "DoorL" "KeepRelative" "KeepRelative" "KeepRelative" true))

(fn GetDoorMeshes
  (return (Utilities|Array|MakeArray (Variables|Default|GetDoorR) (Variables|Default|GetDoorL))))